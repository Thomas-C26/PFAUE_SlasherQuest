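; BP_SlasherAI is a character Blueprint that acts as an interactable quest giver.
; On BeginPlay it applies its MaxWalkSpeed to the movement component.
; When it has a quest, Interact toggles a W_QuestScreen widget, passing itself as QuestGiver.
; Closing the screen restores game-only input but sets the mouse cursor visible, while opening leaves input mode untouched.
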(event `self.ReceiveBeginPlay`
  (set `CharacterMovementComponent.MaxWalkSpeed` (`self.Max Walk Speed`) (`self.CharacterMovement`)))

(event `/Game/Blueprint/_Player/BPI_InteractInterface.Interact`
  (bind _returnvalue (`GameplayStatics.GetPlayerController` 0))
  (if (`self.HasQuest?`)
    (if (`self.QuestScreenOpen?`)
      (`Widget.RemoveFromParent` (`self.QuestScreen`))
      (set `self.QuestScreenOpen?` false)
      (`WidgetBlueprintLibrary.SetInputMode_GameOnly` _returnvalue)
      (set `PlayerController.bShowMouseCursor` true _returnvalue)
      (else
        (bind _returnvalue_2 (`|CreateWidget` "/Game/Blueprint/QuestSystem/W_QuestScreen.W_QuestScreen_C" null self))
        (bind _output_get (set `self.QuestScreen` _returnvalue_2))
        (`UserWidget.AddToViewport` _output_get 0)
        (set `self.QuestScreenOpen?` true)))))

(fn `UserConstructionScript`)