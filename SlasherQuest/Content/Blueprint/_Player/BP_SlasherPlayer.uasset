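; BP_SlasherPlayer is a player character Blueprint with a basic montage-driven attack.
; On BeginPlay it sets the movement component's max walk speed from its Speed variable.
; The Attack input prints a debug string, then plays the attack montage if CanAttack is true.
; CanAttack clears when the montage starts and resets only on its Completed callback, with no handling for interruption.
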(event `self.ReceiveBeginPlay`
  (set `CharacterMovementComponent.MaxWalkSpeed` (`self.Speed`) (`self.CharacterMovement`)))

(event `InputAction|Attack`
  (params (Key :type "Key Structure"))
  (:`Pressed`
    (`KismetSystemLibrary.PrintString` "Attacking")
    (if (`self.CanAttack?`)
      (`|PlayMontage` (`self.Mesh`) "/Game/Characters/Slashers/Animations/M_Attacking.M_Attacking"
        (:`then`
          (set `self.CanAttack?` false))
        (:`OnCompleted`
          (set `self.CanAttack?` true))))))

(fn `UserConstructionScript`)