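; BP_Survivor is an AI survivor character that wanders the level continuously at its maximum run speed.
; On BeginPlay it sets its walk speed to MaxRunSpeed and starts the RandomRoam event.
; RandomRoam uses AI MoveTo toward a random reachable point within a fixed radius of its current location.
; The event re-triggers itself on success, or after a printed message and short delay on failure, forming an endless roam loop.
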(event `self.ReceiveBeginPlay`
  (set `CharacterMovementComponent.MaxWalkSpeed` (`self.Max Run Speed`) (`self.CharacterMovement`))
  (`self.RandomRoam`))

(event `RandomRoam`
  (bind _movementresult (`|AIMoveTo` self (`NavigationSystemV1.K2_GetRandomReachablePointInRadius` (`self.K2_GetActorLocation`) 4000.0 null null) null)
    (:`OnSuccess`
      (`self.RandomRoam`))
    (:`OnFail`
      (`KismetSystemLibrary.PrintString` (`|GetEnumeratorNameAsString` _movementresult))
      (`KismetSystemLibrary.Delay` 0.2)
      (`self.RandomRoam`))))

(fn `UserConstructionScript`)